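; Enemy character Blueprint that casts abilities at a target and reports health, attack range and status through getter functions.
; ActivateAbility stores ability and target, signals cast start, waits the class's CastTime scaled by CastSpeed, then spawns the ability actor and signals cast end.
; Any damage signals an interrupt and briefly sets IsInterrupted, but does not stop a pending cast.
; CancelAbilityActivation is an empty stub.
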(event Custom|Interrupted
  (Default|CallOnAbilityCastInterrupt)
  (Variables|Default|SetIsInterrupted true)
  (Utilities|FlowControl|Delay 1.0)
  (Variables|Default|SetIsInterrupted false))

(event Custom|Start%20Ability
  (Development|PrintString "Abiility Fired")
  (Utilities|FlowControl|Delay (* (Variables|Default|GetCastSpeed) (.CastTime (Utilities|GetClassDefaults (Variables|Default|GetCurrent%20Ability%20To%20Activated)))))
  (CallFunction|AbilityActivated))

(event Game|Damage|EventAnyDamage
  (params (Damage :type Float%20%28single-precision%29) (DamageType :type Damage%20Type%20Object%20Reference) (InstigatedBy :type Controller%20Object%20Reference) (DamageCauser :type Actor%20Object%20Reference))
  (CallFunction|Interrupted))

(event EventTick
  (params (DeltaSeconds :type Float%20%28single-precision%29)))

(event EventBeginPlay)

(fn ConstructionScript)

(fn ActivateAbility
  (params (Ability :type Ability%20Base%20Class%20Reference) (Target :type Actor%20Object%20Reference))
  (Variables|Default|SetCurrentTargetForAbility Target)
  (Variables|Default|SetCurrent%20Ability%20To%20Activated Ability)
  (Default|CallOnAbilityCastStarted)
  (CallFunction|StartAbility))

(fn AbilityActivated
  (bind _self self)
  (Game|SpawnActorfromClass (Variables|Default|GetCurrent%20Ability%20To%20Activated) (Transformation|GetWorldTransform (Variables|Default|GetScene)) "AlwaysSpawn" _self (Variables|Default|GetCurrentTargetForAbility) _self)
  (Default|CallOnAbilityCastEnded))

(fn CancelAbilityActivation)

(fn GetAttackRange
  (return 2e+02 1e+02))

(fn GetHealth
  (return (Variables|Default|GetHealth) (Variables|Default|GetMaxHealth)))

(fn GetIsAlive
  (return (> (Variables|Default|GetHealth) 0.0)))

(fn GetIsCurrentlyInterrupted
  (return (Variables|Default|GetIsInterrupted)))

(fn GetIsPlayer
  (return false))