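; SuckUp is an actor that periodically applies a radial force to components around it, acting as an intermittent suction or force field.
; A looping timer started on BeginPlay flips the IsSucking flag every five seconds.
; While the flag is set, Tick applies a constant-falloff radial force as an acceleration to every component overlapping OuterSphere, centered on the actor and sized to the sphere's scaled radius.
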(event EventBeginPlay
  (bind _returnvalue (Utilities|Time|SetTimerbyFunctionName 0 "TogglingSucking" 5.0 true))
  (Variables|Default|SetToggleSuckTimer _returnvalue))

(event Collision|EventActorBeginOverlap
  (params (OtherActor :type Actor%20Object%20Reference)))

(event EventTick
  (params (DeltaSeconds :type Float%20%28single-precision%29))
  (if (Variables|Default|GetIsSucking)
    (for _array_element (Class|PrimitiveComponent|GetOverlappingComponents (Variables|Default|GetOuterSphere))
      (Physics|AddRadialForce _array_element (Transformation|GetActorLocation) (Components|Sphere|GetScaledSphereRadius (Variables|Default|GetOuterSphere)) (Variables|Default|GetForceStrength) "RIF_Constant" true))))

(fn ConstructionScript)

(fn TogglingSucking
  (Variables|Default|SetIsSucking (not (Variables|Default|GetIsSucking))))